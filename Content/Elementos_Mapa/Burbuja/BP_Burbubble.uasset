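; BP_Burbubble is a map bubble that travels along a spline and restores the first-person character's life while overlapping its capsule.
; Tick advances the sphere along the spline, adding a vertical sine bob driven by world X and elapsed time.
; Speed rises in three tiers as the player's horizontal distance shrinks.
; Capsule overlaps swap the character's looping IncreaseLife and DecreaseLife timers, so life drains after leaving.
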(event OnComponentBeginOverlap(Capsule)
  (params (OverlappedComponent :type Primitive%20Component%20Object%20Reference) (OtherActor :type Actor%20Object%20Reference) (OtherComp :type Primitive%20Component%20Object%20Reference) (OtherBodyIndex :type Integer) (bFromSweep :type Boolean) (SweepResult :type Hit%20Result%20Structure%20%28by%20ref%29))
  (bind _asbp_first_person_character (Utilities|Casting|CastToBP_FirstPersonCharacter OtherActor))
  (Utilities|Time|ClearTimerbyFunctionName _asbp_first_person_character "DecreaseLife")
  (Utilities|Time|SetTimerbyFunctionName _asbp_first_person_character "IncreaseLife" 0.5 true))

(event OnComponentEndOverlap(Capsule)
  (params (OverlappedComponent :type Primitive%20Component%20Object%20Reference) (OtherActor :type Actor%20Object%20Reference) (OtherComp :type Primitive%20Component%20Object%20Reference) (OtherBodyIndex :type Integer))
  (bind _asbp_first_person_character (Utilities|Casting|CastToBP_FirstPersonCharacter OtherActor))
  (Utilities|Time|ClearTimerbyFunctionName _asbp_first_person_character "IncreaseLife")
  (Utilities|Time|SetTimerbyFunctionName _asbp_first_person_character "DecreaseLife" 0.5 true))

(event EventBeginPlay
  (Variables|Default|SetBallStart (Transformation|GetActorLocation)))

(event EventTick
  (params (DeltaSeconds :type Float%20%28single-precision%29))
  (bind _returnvalue (Game|Player|GetPlayerPawn 0))
  (bind _sphere (Variables|Default|GetSphere))
  (bind _returnvalue_2 (Transformation|GetWorldLocation _sphere))
  (bind _returnvalue_3 (Transformation|GetActorLocation _returnvalue))
  (bind (_x _y) (Math|Vector|BreakVector _returnvalue_3))
  (bind (_x_2 _y_2) (Math|Vector|BreakVector _returnvalue_2))
  (bind _returnvalue_4 (Math|Vector|MakeVector _x _y 0.0))
  (bind _returnvalue_5 (Math|Vector|MakeVector _x_2 _y_2 0.0))
  (bind _returnvalue_6 (Math|Vector|Distance(Vector) _returnvalue_4 _returnvalue_5))
  ;[1 1 1] Para alargar el camino, seleccionan la punta y con alt+desplazamiento generan un nuevo punto en el lugar desplazado-
  (Variables|Default|SetAcumulador%20Tiempo (+ DeltaSeconds (Variables|Default|GetAcumulador%20Tiempo)))
  (bind _output_get (Variables|Default|SetPosition_On_Spline (+ (* DeltaSeconds (Variables|Default|GetSpeed_On_Spline)) (Variables|Default|GetPosition_On_Spline))))
  (bind _zfloatingtransform (CallFunction|ZTransformSin (Spline|GetTransformatDistanceAlongSpline (Variables|Default|GetSpline) _output_get "World" false) (Variables|Default|Getamplitud) (Variables|Default|Getfrecuencia) (Variables|Default|GetAcumulador%20Tiempo)))
  (Transformation|SetWorldTransform (Variables|Default|GetSphere) _zfloatingtransform false false)
  (Development|PrintString (Utilities|String|ToString(Vector) _returnvalue_3) true true "(R=0.000000,G=0.660000,B=1.000000,A=1.000000)" 2.0 "posityion")
  (if (> _returnvalue_6 1.2e+03)
    (Variables|Default|SetSpeed_On_Spline 3e+02)
    (elif (> _returnvalue_6 4.5e+02)
      (Variables|Default|SetSpeed_On_Spline 8e+02)
      (else
        (Variables|Default|SetSpeed_On_Spline 1.2e+03))))
  (Development|PrintString (Utilities|String|ToString(Float) (Variables|Default|GetSpeed_On_Spline)) true true "(R=0.000000,G=0.660000,B=1.000000,A=1.000000)" 2.0 "speed")
  (Development|PrintString (Utilities|String|ToString(Float) (Variables|Default|GetPosition_On_Spline)) true true "(R=0.000000,G=0.660000,B=1.000000,A=1.000000)" 2.0 "pos"))

(fn ConstructionScript)

(fn ZTransformSin
  (params (transform :type Transform) (Amplitud :type Float%20%28double-precision%29) (Frecuencia :type Float%20%28double-precision%29) (Time :type Float%20%28double-precision%29))
  (bind (_location _rotation _scale) (Math|Transform|BreakTransform transform))
  (bind (_x _y _z) (Math|Vector|BreakVector _location))
  ;[1 1 1] ping pang pung
  (return (Math|Transform|MakeTransform (Math|Vector|MakeVector _x _y (+ _z (* (Math|Trig|Sin(Degrees) (+ (* _x Frecuencia) Time)) Amplitud))) _rotation _scale)))